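; Runtime FBX importer that brings downloaded models into the GenAI game as mesh actors.
; Server download requests route through the GameState, and completed or skipped downloads feed the custom FBX import with their queue ID.
; After import, it creates a dynamic material on the procedural mesh, selects the actor, loads its downloaded albedo PNG, then advances the local controller's queue.
; Missing meshes trigger import-completion retries; failed material creation loops after a delay.
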(event Custom|SkipDown
  (params (fbxImportManager :type Custom%20FBX%20Import%20Manager%20Object%20Reference) (fbxDownPath :type String) (spawnTrans :type Transform) (RealImportId :type Integer))
  ;[1 1 1] SkipDown
  (Class|CustomFBXImportManager|CustomImportFBXFile fbxImportManager fbxDownPath spawnTrans fbxImportManager RealImportId))

(event Custom|FBX_Import
  (params (fbxImportManager :type Custom%20FBX%20Import%20Manager%20Object%20Reference) (downFbxName :type String) (spawnTrans :type Transform) (RealImportId :type Integer))
  ;[1 1 1] FBX Import
  (Class|CustomFBXImportManager|CustomImportFBXFile downFbxName spawnTrans fbxImportManager RealImportId))

(event Collision|EventActorBeginOverlap
  (params (OtherActor :type Actor%20Object%20Reference)))

(event EventServerModelingDown
  (params (fileName :type String) (SpawnTransform :type Transform) (fbxImporter :type Custom%20FBX%20Import%20Manager%20Object%20Reference) (PlayerController :type Gen%20Ai%20Player%20Controller%20Object%20Reference) (InCustomCurrImportID :type Integer))
  ;[1 1 1] Server Modeling Down
  (bind _asbp_gen_ai_game_state (Utilities|Casting|CastToBP_GenAiGameState (Game|GetGameState)))
  (Default|ServerModelingDown _asbp_gen_ai_game_state fileName SpawnTransform fbxImporter PlayerController InCustomCurrImportID))

(event EventCustomonImportCompleted
  (params (MeshActor :type Custom%20FBX%20Mesh%20Actor%20Object%20Reference) (SceneImporter :type Custom%20FBX%20Scene%20Importer%20Object%20Reference))
  (bind _returnvalue (Actor|GetComponentbyClass MeshActor "/Script/ProceduralMeshComponent.ProceduralMeshComponent"))
  (Utilities|FlowControl|Delay 0.1)
  (bind _output_get (Variables|Default|SetSpawnMeshActor MeshActor))
  (Utilities|IsValid _returnvalue
    (:Is%20Valid
      (bind _returnvalue_2 (Rendering|Material|CreateDynamicMaterialInstance _returnvalue 0 "/Game/Materials/M_BaseMaterial_Inst.M_BaseMaterial_Inst" "None" :!class /Script/Engine.PrimitiveComponent :!label _label))
      (Utilities|IsValid _returnvalue_2
        (:Is%20Valid
          ;[1 1 1] CustomOnImportCompleted
          (Class|FBXImportManager|SelectActor _output_get _returnvalue)
          (Class|FBXImportManager|SelectActor _output_get _returnvalue)
          (bind _asgen_ai_player_controller (Utilities|Casting|CastToGenAiPlayerController (Game|GetPlayerController 0)))
          (bind _returnvalue_3 (Class|GenAiPlayerController|UrlEncode _asgen_ai_player_controller (Variables|/Script/GenAi_Housing.CustomFBXMeshActor|GetFileName _output_get)))
          (bind _texture (|LoadImageFileAsyncNode "E_gd" (Utilities|String|Append "Saved/Download/" _returnvalue_3 "_mesh_albedo.png") "TC_Default" false true false "E_BGRA")
            (:OnSuccess
              (Class|FBXMeshActor|UpdateTextureParameter (Variables|Default|GetSpawnMeshActor) 0 "DiffuseTexture" _texture _returnvalue))
            (:OnFail
              (Development|PrintString "fail" true true "(R=0.000000,G=0.660000,B=1.000000,A=1.000000)" 9999.0)))
          (bind _asgen_ai_player_controller_2 (Utilities|Casting|CastToGenAiPlayerController (Game|GetPlayerController 0)))
          (if (Pawn|IsLocalController _asgen_ai_player_controller_2)
            (Class|GenAiPlayerController|ChkFbxActorQueue _asgen_ai_player_controller_2)))
        (:Is%20Not%20Valid
          (Development|PrintString "NotCreate material. Try Create material" true true "(R=1.000000,G=0.372257,B=0.000000,A=1.000000)" 9999.0)
          (Utilities|FlowControl|Delay 0.1)
          (goto _label))))
    (:Is%20Not%20Valid
      (Development|PrintString "Procedural Not Valid" true true "(R=1.000000,G=0.000000,B=0.945167,A=1.000000)" 99999.0)
      (Class|CustomFBXImportManager|CustomHandleImportCompleted SceneImporter)
      (Development|PrintString "ReImport Try" true true "(R=0.052545,G=1.000000,B=0.000000,A=1.000000)" 9999.0))))

(event EventOnDownComplete
  (params (downFbxName :type String) (spawnTrans :type Transform) (currImportID :type Integer))
  ;[1 1 1] OnDownComplete
  (CallFunction|FBXImport self downFbxName spawnTrans currImportID))

(fn ConstructionScript)