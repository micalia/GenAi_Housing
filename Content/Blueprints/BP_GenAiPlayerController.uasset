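; Player controller that switches the player between the third-person character and a housing pawn for placing AI-generated meshes.
; HousingSystem toggles the cursor, saves housing data to the DB on exit, and has the server possess the housing pawn or the stored character.
; FBX actor creation runs server-side, while LocalModelingDown reuses a saved mesh or downloads mesh and albedo from GameState URLs.
; Transform edits relay through GameState's multicast.
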(event Custom|Multicast_SetActorTransform
  (params (FbxMeshActor :type BP%20Custom%20Fbx%20Actor%20Object%20Reference) (Pos :type Vector) (Rot :type Rotator) (Scale :type Vector))
  (Development|PrintString (Utilities|GetDisplayName FbxMeshActor))
  (Transformation|SetActorTransform FbxMeshActor (Math|Transform|MakeTransform Pos Rot Scale)))

(event Custom|Server_HousingPossess
  (params (Player :type Pawn%20Object%20Reference) (CameraPos :type Vector))
  (bind _asbp_third_person_character (Utilities|Casting|CastToBP_ThirdPersonCharacter Player)
    (:then
      (bind _output_get (Variables|Default|SetprevCharacter _asbp_third_person_character))
      (bind _aswb_player_name (Utilities|Casting|CastToWB_PlayerName (UserInterface|GetWidget (Actor|GetComponentbyClass _output_get "/Script/UMG.WidgetComponent")))
        (:then
          _)
        (:CastFailed
          _))
      (bind _returnvalue (Actor|GetActorOfClass "/Game/Blueprints/BP_HousingPawn.BP_HousingPawn_C"))
      (Variables|/Script/GenAi_Housing.HousingPawn|SetCurrUserName _returnvalue (Utilities|String|ToString(Text) (Variables|/Script/UMG.TextBlock|GetText (Variables|/Script/GenAi_Housing.PlayerNameWidget|GetPlayerNameTxt _aswb_player_name))))
      (Transformation|SetActorLocation _returnvalue CameraPos false false)
      (Pawn|Possess _returnvalue))
    (:CastFailed
      (Pawn|Possess (Variables|Default|GetprevCharacter)))))

(event Custom|FileDown
  (params (fileName :type String) (spawnTrans :type Transform) (fbxImporter :type Custom%20FBX%20Import%20Manager%20Object%20Reference) (PlayerControoler :type Gen%20Ai%20Player%20Controller%20Object%20Reference))
  (bind _returnvalue (Class|GenAiPlayerController|UrlEncode fileName))
  (bind _asgen_ai_game_state (Utilities|Casting|CastToGenAiGameState (Game|GetGameState)))
  (Utilities|FlowControl|Sequence
    (:then_0
      (Class|CustomFBXImportManager|DownFbxFileCPP fbxImporter (Utilities|String|Append (Variables|/Script/GenAi_Housing.HttpRequestActor|GetAI_FBX_FULL_PATH (Variables|/Script/GenAi_Housing.GenAiGameState|GetHttpRequestActor _asgen_ai_game_state)) _returnvalue "_mesh.fbx") (Utilities|String|Append (Class|BlueprintPathsLibrary|ProjectSavedDir) "Download/" _returnvalue "_mesh.fbx") _returnvalue spawnTrans))
    (:then_1
      (Class|CustomFBXImportManager|DownTextureFileCPP fbxImporter (Utilities|String|Append (Variables|/Script/GenAi_Housing.HttpRequestActor|GetAI_TEXTURE_FULL_PATH (Variables|/Script/GenAi_Housing.GenAiGameState|GetHttpRequestActor _asgen_ai_game_state)) _returnvalue "_mesh_albedo.png") (Utilities|String|Append (Class|BlueprintPathsLibrary|ProjectSavedDir) "Download/" _returnvalue "_mesh_albedo.png")))))

(event Custom|Server_SetActorTransform
  (params (FbxMeshActor :type BP%20Custom%20Fbx%20Actor%20Object%20Reference) (Pos :type Vector) (Rot :type Rotator) (Scale :type Vector))
  (bind _asbp_gen_ai_game_state (Utilities|Casting|CastToBP_GenAiGameState (Game|GetGameState)))
  (Default|MulticastSetActorTransform _asbp_gen_ai_game_state FbxMeshActor Pos Rot Scale))

(event Custom|Server_SetCurrSelectInfoAndCreateFbxActor
  (params (ObjPrompt :type String) (MakeTimeStamp :type String) (SpawnLoc :type Vector) (FbxImporter :type Custom%20FBX%20Import%20Manager%20Object%20Reference) (PlayController :type BP%20Gen%20Ai%20Player%20Controller%20Object%20Reference) (ObjIndex :type Integer))
  (Class|CustomFBXImportManager|CreateFBXActorinServer FbxImporter (Utilities|String|Append MakeTimeStamp "_" ObjPrompt) SpawnLoc FbxImporter PlayController ObjIndex))

(event EventHousingSystem
  (bind _returnvalue (Game|Player|GetPlayerPawn 0))
  (bind _returnvalue_2 (Game|GetPlayerController 0))
  (Utilities|Casting|CastToBP_ThirdPersonCharacter _returnvalue
    (:then
      (Variables|/Script/Engine.PlayerController|SetbShowMouseCursor _returnvalue_2 true))
    (:CastFailed
      (bind _asbp_housing_pawn (Utilities|Casting|CastToBP_HousingPawn _returnvalue)
        (:then
          _)
        (:CastFailed
          _))
      (Class|GenAiPlayerController|ServerInsertObjDatatoDB (Variables|/Script/GenAi_Housing.HousingPawn|GetCurrUserName _asbp_housing_pawn))
      (Variables|/Script/Engine.PlayerController|SetbShowMouseCursor _returnvalue_2 false)))
  (CallFunction|ServerHousingPossess _returnvalue (Transformation|GetActorLocation (Game|GetPlayerCameraManager 0))))

(event EventTick
  (params (DeltaSeconds :type Float%20%28single-precision%29)))

(event EventLocalModelingDown
  (params (FileName :type String) (SpawnTrans :type Transform) (FbxImportManager :type Custom%20FBX%20Import%20Manager%20Object%20Reference) (PlayerController :type Gen%20Ai%20Player%20Controller%20Object%20Reference))
  (if (Ability|HasAuthority)
    _
    (else
      (Utilities|FlowControl|Delay 2.0)))
  (CallFunction|FileExistCheck FileName SpawnTrans FbxImportManager PlayerController))

(fn ConstructionScript)

(fn FileExistCheck
  (params (fileName :type String) (spawnTrans :type Transform) (fbxImportManager :type Custom%20FBX%20Import%20Manager%20Object%20Reference) (playerController :type Gen%20Ai%20Player%20Controller%20Object%20Reference))
  (bind _returnvalue (Class|BlueprintPathsLibrary|ProjectSavedDir))
  (bind _returnvalue_2 (Utilities|String|Append _returnvalue "Download/" fileName "_mesh.fbx"))
  (if (Class|BlueprintPathsLibrary|FileExists _returnvalue_2)
    (bind _asbp_custom_fbx_importer (Utilities|Casting|CastToBP_CustomFbxImporter fbxImportManager))
    (Default|SkipDown _asbp_custom_fbx_importer fbxImportManager _returnvalue_2 (.Location (Math|Transform|BreakTransform spawnTrans)))
    (else
      (CallFunction|FileDown fileName spawnTrans fbxImportManager playerController))))