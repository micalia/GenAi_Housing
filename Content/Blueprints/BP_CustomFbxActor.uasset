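; BP_CustomFbxActor is an actor, apparently for custom FBX imports, that draws its current import ID as debug text at its location every tick.
; When a component is selected, it stores the mesh, switches its collision object type to GameTraceChannel1 and creates a dynamic material instance from M_BaseMaterial_Inst.
; Procedural mesh replication, bounds-based rescaling and translation gizmo attachment exist only as disconnected, never-executed graphs.
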(event EventBeginPlay)

(event Collision|EventActorBeginOverlap
  (params (OtherActor :type Actor%20Object%20Reference)))

(event EventTick
  (params (DeltaSeconds :type Float%20%28single-precision%29))
  (Rendering|Debug|DrawDebugString (Transformation|GetActorLocation) (Utilities|String|Append "CuureID : " (Utilities|String|ToString(Integer) (Variables|Default|GetCustomCurrentImportID))) 0 "(R=0.189559,G=0.000000,B=0.255208,A=1.000000)" 0.1))

(event EventOnComponentSelected
  (params (MeshComponent :type Procedural%20Mesh%20Component%20Object%20Reference))
  (bind _output_get (Variables|Default|SetCurrComponent MeshComponent))
  (Collision|SetCollisionObjectType _output_get "ECC_GameTraceChannel1")
  ;[1 1 1] OnComponentSelected
  (Rendering|Material|CreateDynamicMaterialInstance _output_get 0 "/Game/Materials/M_BaseMaterial_Inst.M_BaseMaterial_Inst" "None" :!class /Script/Engine.PrimitiveComponent))

(fn ConstructionScript)