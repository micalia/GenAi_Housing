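; BP_FBXMeshActor is an actor for an FBX mesh that can be selected by component.
; The construction script applies SpawnScale to the actor.
; OnComponentSelected stores the selected component as CurrComponent and switches its collision object type to the GameTraceChannel1 custom channel.
; All other logic is disconnected and never runs: debug prints, procedural mesh replication, bounds-based rescaling and attachment to BP_TranslationGizmo_Example.
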(event EventBeginPlay)

(event Collision|EventActorBeginOverlap
  (params (OtherActor :type Actor%20Object%20Reference)))

(event EventTick
  (params (DeltaSeconds :type Float%20%28single-precision%29)))

(event EventOnComponentSelected
  (params (MeshComponent :type Procedural%20Mesh%20Component%20Object%20Reference))
  (bind _output_get (Variables|Default|SetCurrComponent MeshComponent))
  (Collision|SetCollisionObjectType _output_get "ECC_GameTraceChannel1"))

(fn ConstructionScript
  (Transformation|SetActorScale3D (Variables|Default|GetSpawnScale)))